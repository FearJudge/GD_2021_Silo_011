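; Enemy entity character that chases the player, with trail and shadow effects activated at BeginPlay.
; A one-time 3000-unit distance check at BeginPlay or a PawnSensing sighting sets IsSeeingPlayer, which is never cleared, and starts AIMoveTo toward the player.
; Timer-driven glitch events for random short teleports and a mesh visibility swap are present but never triggered.
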(event `self.ReceiveBeginPlay`
  (`ActorComponent.Activate` (`self.FX_Trails`) false)
  (`ActorComponent.Activate` (`self.FX_CreeperShadow_v4`) false)
  (`self.CheckForPlayerInRadius`))

(event `CheckForPlayerInRadius`
  (bind _returnvalue_location (`KismetMathLibrary.BreakTransform` (`self.GetTransform`)))
  (bind _returnvalue_location_2 (`KismetMathLibrary.BreakTransform` (`self.GetTransform` (`GameplayStatics.GetPlayerCharacter` 0))))
  (if (< (`KismetMathLibrary.Abs` (`KismetMathLibrary.Vector_Distance` _returnvalue_location _returnvalue_location_2)) 3000.0)
    (set `self.isSeeingPlayer` true :!label _label)
    (`self.FollowPlayer`)))

(event `self.PawnSensing.OnSeePawn`
  (params (Pawn :type "Pawn Object Reference"))
  (goto _label))

(event `FollowPlayer`
  (if (`self.isSeeingPlayer`)
    (`|AIMoveTo` self (0.0 0.0 0.0) (`GameplayStatics.GetPlayerCharacter` 0))))

(event `MovementGlitch`
  (bind _returnvalue (`KismetMathLibrary.RandomFloatInRange` -100.0 100.0))
  (bind _capsulecomponent (`self.CapsuleComponent`))
  (bind (_returnvalue_x _returnvalue_y _returnvalue_z) (`KismetMathLibrary.BreakVector` (`SceneComponent.K2_GetComponentLocation` _capsulecomponent)))
  (bind _output_get (set `self.RandomTime` (`KismetMathLibrary.RandomFloatInRange` 1.0 4.0)))
  (bind _returnvalue_2 (`self.K2_TeleportTo` (`KismetMathLibrary.MakeVector` (+ _returnvalue _returnvalue_x) (+ _returnvalue _returnvalue_y) _returnvalue_z) (`SceneComponent.K2_GetComponentRotation` _capsulecomponent)))
  (`KismetSystemLibrary.PrintString` "false" _returnvalue_2)
  (`KismetSystemLibrary.K2_SetTimerDelegate` (delegate `MovementGlitch`) _output_get))

(event `VisibilityGlitch`
  (`KismetSystemLibrary.K2_SetTimerDelegate` (delegate `SetTimer`) (stale `SetTimer` _output_get) true))

(event `SetTimer`
  (bind _output_get (set `self.RandomTime` (`KismetMathLibrary.RandomFloatInRange` 1.0 4.0)))
  (`SceneComponent.SetVisibility` (`self.CharacterMesh1`) true false)
  (`SceneComponent.SetVisibility` (`self.Mesh`) false false))

(fn `SetVisibility`
  (`SceneComponent.SetVisibility` (`self.CharacterMesh1`) true false)
  (`SceneComponent.SetVisibility` (`self.Mesh`) false false))

(fn `UserConstructionScript`)