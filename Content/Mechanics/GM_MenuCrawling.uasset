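; Game mode for the main menu that shows the menu widget and manages saved player preferences.
; On BeginPlay it passes the first level name to the widget, loads options into HorrorSiloGameInstance, then applies audio mixing.
; Saving reads the calling widget's BGM and SFX sliders, writes a SAVE_Preferences slot with the FS flag always true, then reloads it.
; Loading copies only the two volumes and flags that a save existed.
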(event `self.ReceiveBeginPlay`
  (bind _returnvalue (`|CreateWidget` "/Game/Mechanics/UIPieces/UI_MENU_MainMenu.UI_MENU_MainMenu_C" (`GameplayStatics.GetPlayerController` 0)))
  (set `/Game/Mechanics/UIPieces/UI_MENU_MainMenu.LevelName` (`self.FirstLevelName`) _returnvalue)
  (`UserWidget.AddToViewport` _returnvalue 0)
  (`self.LoadAndAssignOptions`)
  (bind _ashorror_silo_game_instance (cast `/Game/Mechanics/HorrorSiloGameInstance` (`GameplayStatics.GetGameInstance`)))
  (`/Game/Mechanics/HorrorSiloGameInstance.SetAudioMixing` _ashorror_silo_game_instance))

(fn `LoadAndAssignOptions`
  (locals (OptionsName :type String :default "Silo11_Preferences"))
  (bind _ashorror_silo_game_instance (cast `/Game/Mechanics/HorrorSiloGameInstance` (`GameplayStatics.GetGameInstance`) :!pure true))
  (bind _returnvalue (`GameplayStatics.LoadGameFromSlot` (`local.OptionsName`)))
  (bind _assave_preferences (cast `/Game/Mechanics/SAVE_Preferences` _returnvalue))
  (set `/Game/Mechanics/HorrorSiloGameInstance.VolumeSFX` (`/Game/Mechanics/SAVE_Preferences.Volume_SFX` _assave_preferences) _ashorror_silo_game_instance)
  (set `/Game/Mechanics/HorrorSiloGameInstance.VolumeBGM` (`/Game/Mechanics/SAVE_Preferences.Volume_BGM` _assave_preferences) _ashorror_silo_game_instance)
  (set `/Game/Mechanics/HorrorSiloGameInstance.LoadExisted` true _ashorror_silo_game_instance))

(fn `SaveLoadOptionsData`
  (params (Load :type Boolean) (CalledFrom :type "/Game/Mechanics/UIPieces/UI_MENU_MainMenu Object Reference"))
  (locals (LocalFS :type Boolean) (LocalBGM :type "Float (double-precision)") (LocalSFX :type "Float (double-precision)") (OptionsName :type String :default "Silo11_Preferences"))
  (if Load
    (`self.LoadAndAssignOptions` :!label _label)
    (else
      (bind _returnvalue (`GameplayStatics.CreateSaveGameObject` "/Game/Mechanics/SAVE_Preferences.SAVE_Preferences_C"))
      (if (`KismetSystemLibrary.IsValid` CalledFrom)
        (`|ExecutionSequence`
          (:`then_0`
            (set `local.LocalFS` true))
          (:`then_1`
            (set `local.LocalBGM` (`Slider.GetNormalizedValue` (`/Game/Mechanics/UIPieces/UI_MENU_MainMenu.ValueSlider` CalledFrom))))
          (:`then_2`
            (set `local.LocalSFX` (`Slider.GetNormalizedValue` (`/Game/Mechanics/UIPieces/UI_MENU_MainMenu.ValueSlider_1` CalledFrom))))
          (:`then_3`
            (`/Game/Mechanics/SAVE_Preferences.SetData` _returnvalue (`local.LocalFS`) (`local.LocalSFX`) (`local.LocalBGM`))
            (`GameplayStatics.SaveGameToSlot` _returnvalue (`local.OptionsName`))
            (goto _label)))))))

(fn `UserConstructionScript`)