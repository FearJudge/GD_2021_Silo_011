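; GM_Silo13 is the Silo 13 horror game mode and central hub for dialogue, objectives, keywords, inventory, puzzles and save/load.
; Data tables fill items, objectives and keywords at construction, and a random session seed randomizes the numpad and light puzzles.
; Queued discussions play through a pausable line loop gated by radio comms and branch choices.
; Line effects call player functions, while temporary "delirious" objectives remove themselves after a short delay.
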(event `DeliriusMessage`
  (bind _objectives (`self.Objectives`))
  (`KismetSystemLibrary.Delay` (`KismetMathLibrary.RandomFloatInRange` 2.0 4.0))
  (bind _loop_item (`/Game/Mechanics/MACRO_Custom.CFL_ForEachLoopReversed` _objectives)
    (:`Loop Bodym`
      (if (`.IsDelirius_5_071C5772447D37DDA4F7A592606900A5` (break `/Game/Mechanics/Structures/DAT_Objectives` _loop_item))
        (`KismetArrayLibrary.Array_RemoveItem` _objectives _loop_item)))))

(event `DialogueRunner`
  (params (DiscussionLines :type "Array of /Game/Mechanics/Structures/DAT_DiscussionLine Structure") (Discussion :type String))
  (bind _paused_cfl (`self.PAUSED_CFL`))
  (bind _branch (`self.Branch`))
  (bind _discussionsrun (`self.DiscussionsRun`))
  (bind _discussions (`self.Discussions`))
  (bind _isinradiocomms (`/Game/Mechanics/BP_Player.IsInRadioComms` (`self.Player`)))
  (bind _hud_dialogue (`/Game/Mechanics/BP_Player.HUD_Dialogue` (`self.Player`)))
  (bind _returnvalue (not _isinradiocomms))
  (set `self.IsTalking` true)
  (if (and (`KismetArrayLibrary.Array_Contains` _discussionsrun Discussion) (`KismetStringLibrary.Contains` Discussion "Optional"))
    (set `self.Branch` 1)
    (else
      (`KismetArrayLibrary.Array_Add` _discussionsrun Discussion)))
  (bind _arrayelement (`/Game/Mechanics/MACRO_Custom.CFL_ForEachLoopDelayed` DiscussionLines :!label _label)
    (:`Body`
      (switch `/Game/Mechanics/Structures/ENUM_DialogueType` (`.SpeakLogic_21_BB6CC9DF4F207F0E7CEA558DA3265530` (break `/Game/Mechanics/Structures/DAT_DiscussionLine` _arrayelement))
        (:`NewEnumerator0`
          (if _isinradiocomms
            (set `self.PAUSED_CFL` true :!label _label_2)
            (`|ExecutionSequence` :!label _label_3
              (:`then_0`
                (`self.ResumeDialogue`))
              (:`then_1`
                (bind (_out _speakingin) (`/Game/Mechanics/HorrorSiloGameInstance.GetSpeakerDisplayName` (cast `/Game/Mechanics/HorrorSiloGameInstance` (`GameplayStatics.GetGameInstance`) :!pure true) (`.DialogueGiver_9_D8B28AB74DAF948C25D59884FE980C0F` (break `/Game/Mechanics/Structures/DAT_DiscussionLine` _arrayelement)) true)))
              (:`then_2`
                (`/Game/Mechanics/UIPieces/UI_Dialogue.SetDialogue` _hud_dialogue _out (break `/Game/Mechanics/Structures/DAT_DiscussionLine` _arrayelement) _speakingin)
                (`GameplayStatics.PlaySound2D` (`.VoiceLine_5_14FC71B54EDEF8D2169378B46B44AABB` (break `/Game/Mechanics/Structures/DAT_DiscussionLine` _arrayelement)) 1.0 1.0 0.0 null null))
              (:`then_3`
                (if (`|EnumInequality` (`.LineAddEffect_15_F010C6BB421F8113304D92AF2EE86431` (break `/Game/Mechanics/Structures/DAT_DiscussionLine` _arrayelement)) "NewEnumerator3")
                  (`self.CallPlayerFunction` (`.LineAddEffect_15_F010C6BB421F8113304D92AF2EE86431` (break `/Game/Mechanics/Structures/DAT_DiscussionLine` _arrayelement)) (`.LineEffectParam_18_5B7C8943464E9D87A93CC5BD83703656` (break `/Game/Mechanics/Structures/DAT_DiscussionLine` _arrayelement))))))
            (else
              (`self.SkipDialogue` :!label _label_4))))
        (:`NewEnumerator1`
          (if _isinradiocomms
            (goto _label_4)
            (else
              (goto _label_2))))
        (:`NewEnumerator2`
          (set `self.PAUSED_CFL` false :!label _label_5)
          (goto _label_3))
        (:`NewEnumerator3`
          (if _returnvalue
            (`self.PauseDialogue` false)
            (elif _paused_cfl
              (goto _label_5)
              (else
                (`self.StopSkips`)))))
        (:`NewEnumerator4`
          (if _returnvalue
            (`self.SkipDialogue` :!label _label_6)
            (else
              (goto _label_5))))
        (:`NewEnumerator5`
          (if (and _isinradiocomms _paused_cfl)
            (goto _label_3)
            (else
              (goto _label_6))))
        (:`NewEnumerator6`
          (if (== _branch 1)
            (goto _label_5)
            (else
              (goto _label_6))))
        (:`NewEnumerator7`
          (if (== _branch 2)
            (goto _label_5)
            (else
              (goto _label_6))))
        (:`NewEnumerator8`
          (if (== _branch 3)
            (goto _label_5)
            (else
              (goto _label_6))))
        (:`NewEnumerator9`
          (if (== _branch 4)
            (goto _label_5)
            (else
              (goto _label_6))))
        (:`NewEnumerator10`
          (if (== _branch 0)
            (`self.PauseDialogue` true)
            (else
              (goto _label_5))))
        (:`NewEnumerator11`
          (if (== _branch 0)
            (goto _label_5)
            (else
              (goto _label_6))))))
    (:`Complete`
      (`/Game/Mechanics/UIPieces/UI_Dialogue.UnsetDialogue` _hud_dialogue)
      (set `self.IsTalking` false)
      (if (> (`KismetArrayLibrary.Array_Length` _discussions) 0)
        (`self.DiscussionRunThrough` (`|GetArrayItem` _discussions))
        (`KismetArrayLibrary.Array_Remove` _discussions)))))

(event `ResumeDialogue`
  (bind _player (`self.Player`))
  (`|ExecutionSequence`
    (:`then_0`
      (goto _label :!via `ResumeDialogue`))
    (:`then_1`
      (goto _label :!via `StopSkipping`))
    (:`then_2`
      (if (`|EnumEquality` (`/Game/Mechanics/BP_Player.PlayerControlMode` _player) "NewEnumerator6")
        (set `/Game/Mechanics/BP_Player.PlayerControlMode` "NewEnumerator0" _player)))))

(event `DiscussionRunThrough`
  (params (DiscussionID :type String))
  (bind _discussionsearch (`self.DiscussionSearch`))
  (bind (_value _returnvalue) (`BlueprintMapLibrary.Map_Find` (`self.DiscussionIDMap`) _discussionsearch))
  (if (`self.IsTalking`)
    (`KismetArrayLibrary.Array_AddUnique` (`self.Discussions`) DiscussionID)
    (else
      (for (_array_element _array_index) (`KismetStringLibrary.ParseIntoArray` DiscussionID "=")
        (if (== _array_index 0)
          (set `self.DiscussionSearch` (`KismetStringLibrary.Replace` _array_element " " "_"))
          (else
            (`/Game/Mechanics/HorrorSiloGameInstance.ParseDialogueForSpecialCases` (cast `/Game/Mechanics/HorrorSiloGameInstance` (`GameplayStatics.GetGameInstance`) :!pure true) _array_element))))
      (if _returnvalue
        (`self.DialogueRunner` (`.DiscussionLines_9_4F73DE6D4087F1AE9D6FBE8ED56A6E95` (break `/Game/Mechanics/Structures/DAT_Discussion` _value)) (break `/Game/Mechanics/Structures/DAT_Discussion` _value))
        (else
          (bind _discussion (`self.ReturnDiscussionViaDirectID` _discussionsearch))
          (`self.DialogueRunner` (`.DiscussionLines_9_4F73DE6D4087F1AE9D6FBE8ED56A6E95` (break `/Game/Mechanics/Structures/DAT_Discussion` _discussion)) (break `/Game/Mechanics/Structures/DAT_Discussion` _discussion)))))))

(event `PauseDialogue`
  (params (ShowBranches :type Boolean))
  (bind _branchchoices (`self.BranchChoices`))
  (bind _player (`self.Player`))
  (bind _hud_dialogue (`/Game/Mechanics/BP_Player.HUD_Dialogue` _player))
  (if ShowBranches
    (bind _allfalse (`/Game/Mechanics/UIPieces/UI_Dialogue.CreateChoices` _hud_dialogue (`|GetArrayItem` _branchchoices) (`|GetArrayItem` _branchchoices 1) (`|GetArrayItem` _branchchoices 2) (`|GetArrayItem` _branchchoices 3)))
    (if _allfalse
      (`self.SkipDialogue`)
      (else
        (set `/Game/Mechanics/BP_Player.PlayerControlMode` "NewEnumerator6" _player)
        (set `self.PAUSED_CFL` true :!label _label_7)
        (`self.StopSkips`)
        (goto _label :!via `PauseDialogue`)))
    (else
      (`/Game/Mechanics/UIPieces/UI_Dialogue.UnsetDialogue` _hud_dialogue)
      (goto _label_7))))

(event `SkipDialogue`
  (`/Game/Mechanics/UIPieces/UI_Dialogue.UnsetDialogue` (`/Game/Mechanics/BP_Player.HUD_Dialogue` (`self.Player`)))
  (goto _label :!via `SkipDialogue`))

(event `StopSkips`
  (goto _label :!via `StopSkipping`))

(event `AdvanceDialogueOne`
  (goto _label :!via `AdvanceOncem`))

(event `self.ReceiveBeginPlay`
  (bind _returnvalue (`GameplayStatics.GetPlayerController` 0))
  (bind _shouldload (`/Game/Mechanics/HorrorSiloGameInstance.ShouldLoad` (cast `/Game/Mechanics/HorrorSiloGameInstance` (`GameplayStatics.GetGameInstance`) :!pure true)))
  (`|ExecutionSequence`
    (:`then_0`
      ;[1 1 1] CreateAndStorePuzzles
      (`|ExecutionSequence`
        (:`then_0`
          (if _shouldload
            (`self.SaveLoad` true)))
        (:`then_1`
          (bind _returnvalue_2 (`|CreateWidget` "/Game/Mechanics/UIPieces/UI_4-DigitLock.UI_4-DigitLock_C" _returnvalue))
          (set `self.Puzzle_NumPadOne` _returnvalue_2)
          (`/Game/Mechanics/UIPieces/UI_4-DigitLock.RandomizeSolution` (`self.Puzzle_NumPadOne`) (`self.GameSessionSeed`)))
        (:`then_2`
          (bind _returnvalue_3 (`|CreateWidget` "/Game/Mechanics/UIPieces/UI_LightPuzzle.UI_LightPuzzle_C" _returnvalue))
          (set `self.PuzzleLightPuzzleOne` _returnvalue_3)
          (`/Game/Mechanics/UIPieces/UI_LightPuzzle.RandomizeSolution` (`self.PuzzleLightPuzzleOne`) (`self.GameSessionSeed`)))
        (:`then_3`
          (`KismetSystemLibrary.DelayUntilNextTick`)
          (if (not _shouldload)
            (`self.DiscussionRunThrough` "MainDialogue_DemoIntro")))))
    (:`then_1`
      ;[1 1 1] Create Other Game Logic
      (`|ExecutionSequence`
        (:`then_0`
          (bind _ashorror_silo_game_instance (cast `/Game/Mechanics/HorrorSiloGameInstance` (`GameplayStatics.GetGameInstance`)))
          (`/Game/Mechanics/HorrorSiloGameInstance.SetAudioMixing` _ashorror_silo_game_instance))))))

(event `GM_Silo13_AutoGenFunc`
  (bind _ashorror_silo_game_instance (cast `/Game/Mechanics/HorrorSiloGameInstance` (`GameplayStatics.GetGameInstance`)))
  (if (`/Game/Mechanics/HorrorSiloGameInstance.ShouldLoad` _ashorror_silo_game_instance)
    (`KismetSystemLibrary.DelayUntilNextTick`)
    (`self.SaveLoad` true 0 true)
    (`KismetSystemLibrary.PrintString` "Level Part Loaded")))

(fn `AddInventoryItem`
  (params (ItemID :type String))
  (bind _inventory (`self.Inventory`))
  (for (_array_element _array_index) _inventory
    (if (`KismetStringLibrary.EqualEqual_StrStr` _array_element)
      (`KismetArrayLibrary.Array_Set` _inventory _array_index ItemID)
      (return))))

(fn `AddRemoveObjectives`
  (params (ObjectiveID :type String) (AddOnly :type Boolean) (RemoveOnly :type Boolean) (AddTemporary :type Boolean))
  (locals (ObjectiveDat :type "/Game/Mechanics/Structures/DAT_Objectives Structure") (NameToCheck :type Name :default "None"))
  (bind _objectives (`self.Objectives`))
  (bind _objectivedat (`local.ObjectiveDat`))
  (bind (_objectivedat_objectivename _objectivedat_isdelirius) (break `/Game/Mechanics/Structures/DAT_Objectives` (`local.ObjectiveDat`)))
  (for _index (range 6)
    (`|ExecutionSequence`
      (:`then_0`
        (switch `int` _index
          (:`0`
            (set `local.NameToCheck` (`KismetStringLibrary.Conv_StringToName` ObjectiveID)))
          (:`1`
            (set `local.NameToCheck` (`KismetStringLibrary.Conv_StringToName` (`KismetStringLibrary.Concat_StrStr` ObjectiveID "(A)"))))
          (:`2`
            (set `local.NameToCheck` (`KismetStringLibrary.Conv_StringToName` (`KismetStringLibrary.Concat_StrStr` ObjectiveID "(B)"))))
          (:`3`
            (set `local.NameToCheck` (`KismetStringLibrary.Conv_StringToName` (`KismetStringLibrary.Concat_StrStr` ObjectiveID "(C)"))))
          (:`4`
            (set `local.NameToCheck` (`KismetStringLibrary.Conv_StringToName` (`KismetStringLibrary.Concat_StrStr` ObjectiveID "(D)"))))))
      (:`then_1`
        (bind _returnvalue (`|GetDataTableRow` (`self.ObjectiveData`) (`local.NameToCheck`))
          (:`then`
            (if AddTemporary
              (bind (_objectivename _isdelirius _markcompletedon) (break `/Game/Mechanics/Structures/DAT_Objectives` _returnvalue))
              (set `local.ObjectiveDat` (make `/Game/Mechanics/Structures/DAT_Objectives` _objectivename true _markcompletedon))
              (else
                (set `local.ObjectiveDat` _returnvalue)))
            (if (and _objectivedat_isdelirius (not (`KismetArrayLibrary.Array_Contains` (`self.Objectives`) (`local.ObjectiveDat`))))
              (`self.DeliriusMessage`))
            (if AddOnly
              (`KismetArrayLibrary.Array_Add` _objectives _objectivedat)
              (elif RemoveOnly
                (`KismetArrayLibrary.Array_RemoveItem` _objectives _objectivedat)
                (else
                  (`KismetArrayLibrary.Array_RemoveItem` _objectives _objectivedat)
                  (`KismetArrayLibrary.Array_Add` _objectives _objectivedat))))))))))

(fn `CallPlayerFunction`
  (params (Function :type "/Game/Mechanics/Structures/ENUM_PlayerFuncs Enum" :default "NewEnumerator0") (Parameter :type String))
  (bind _player (`self.Player`))
  (bind _inventory (`self.Inventory`))
  (bind _flags (`self.Flags`))
  (`/Engine/EditorBlueprintResources/StandardMacros.IsValid` (`self.Player`)
    (:`Is Valid`
      (switch `/Game/Mechanics/Structures/ENUM_PlayerFuncs` Function
        (:`NewEnumerator0`
          (`/Game/Mechanics/BP_Player.ToggleINVENTORY` _player true false))
        (:`NewEnumerator1`
          (`/Game/Mechanics/BP_Player.ToggleMEMO` _player))
        (:`NewEnumerator2`
          (`KismetArrayLibrary.Array_Set` _inventory (`KismetArrayLibrary.Array_Find` _inventory Parameter)))
        (:`NewEnumerator5`
          (`self.DiscussionRunThrough` Parameter))
        (:`NewEnumerator6`
          (`self.DiscoverKeyword` Parameter))
        (:`NewEnumerator7`
          (`self.SaveLoad` false))
        (:`NewEnumerator8`
          (`self.AddRemoveObjectives` Parameter))
        (:`NewEnumerator9`
          (if (`KismetStringLibrary.IsNumeric` Parameter)
            (`self.MarkObjectiveNumCompleted` (`KismetStringLibrary.Conv_StringToInt` Parameter))))
        (:`NewEnumerator10`
          (`self.RemoveKeyword` Parameter))
        (:`NewEnumerator11`
          (if (`BlueprintMapLibrary.Map_Contains` _flags Parameter)
            (`BlueprintMapLibrary.Map_Add` _flags Parameter true)))))
    (:`Is Not Valid`
      (`KismetSystemLibrary.PrintString` "Called Function before Assigning Player to GM!"))))

(fn `DiscoverKeyword`
  (params (Keyword :type String))
  (for (_array_element _array_index) (`self.Keywords`)
    (bind (_keyword _isunlocked _requiresfocus _lockdiscoverability) (break `/Game/Mechanics/Structures/DAT_Keywords` _array_element))
    ;[1 1 1] Check if Exists
    (if (`KismetStringLibrary.EqualEqual_StrStr` _keyword Keyword)
      ;[1 1 1] Check if Already Owned
      (if (or _isunlocked _lockdiscoverability)
        (return)
        (else
          (`/Game/Mechanics/BP_Player.PlayNewDiscoveredKeyword` (`self.Player`) Keyword)
          (`KismetArrayLibrary.Array_Set` (`self.Keywords`) _array_index (make `/Game/Mechanics/Structures/DAT_Keywords` _keyword true _requiresfocus)))))))

(fn `GetInventorySlotIcon`
  (params (Index :type Integer))
  (returns (Icon :type "Texture2D Object Reference"))
  (for _array_element (`self.Items`)
    (if (`KismetStringLibrary.EqualEqual_StrStr` (break `/Game/Mechanics/Structures/DAT_ItemDetails` _array_element) (`|GetArrayItem` (`self.Inventory`) Index))
      (return (`.ItemImage_9_91763C5D45B7366BB0C384BD22C66EB1` (break `/Game/Mechanics/Structures/DAT_ItemDetails` _array_element)))))
  (return "/Game/Sprites/Inventory_Base.Inventory_Base"))

(fn `MarkObjectiveNumCompleted`
  (params (CompletionIndex :type Integer))
  (bind _objectives (`self.Objectives`))
  (for _array_element _objectives
    (if (== (`.MarkCompletedOn_8_61A3D20145434BAB5E7248B9507E3F91` (break `/Game/Mechanics/Structures/DAT_Objectives` _array_element)) CompletionIndex)
      (`KismetArrayLibrary.Array_RemoveItem` _objectives _array_element))))

(fn `OpenPuzzleInterface`
  (params (PuzzleID :type Integer))
  (returns (Puzzle :type "/Game/Mechanics/UIPieces/UI_PuzzleBorder Object Reference"))
  (locals (PuzzleBorder :type "/Game/Mechanics/UIPieces/UI_PuzzleBorder Object Reference"))
  (bind _puzzleborder (`local.PuzzleBorder`))
  (bind _puzzleborder_2 (`local.PuzzleBorder`))
  (if (not (`self.PuzzleBorderActive`))
    (bind _returnvalue (`KismetSystemLibrary.LoadClassAsset_Blocking` "/Game/Mechanics/UIPieces/UI_PuzzleBorder.UI_PuzzleBorder_C"))
    (bind _returnvalue_2 (`|GenericCreateObject` _returnvalue))
    (set `self.PuzzleBorderActive` true)
    (bind _asui_puzzle_border (cast `/Game/Mechanics/UIPieces/UI_PuzzleBorder` _returnvalue_2 :!pure true))
    (set `local.PuzzleBorder` _asui_puzzle_border)
    (`UserWidget.AddToViewport` _asui_puzzle_border 0)
    (`|ExecutionSequence`
      (:`then_0`
        (switch `int` PuzzleID
          (:`0`
            (`/Game/Mechanics/UIPieces/UI_PuzzleBorder.SetUpPuzzle` _puzzleborder_2 "Numpad" (`self.Puzzle_NumPadOne`))
            (`/Game/Mechanics/UIPieces/UI_PuzzleBorder.InitializeSystems` _puzzleborder_2))
          (:`1`
            (`/Game/Mechanics/UIPieces/UI_PuzzleBorder.SetUpPuzzle` _puzzleborder "Lightpad" (`self.PuzzleLightPuzzleOne`))
            (`/Game/Mechanics/UIPieces/UI_PuzzleBorder.InitializeSystems` _puzzleborder))))
      (:`then_1`
        (`/Game/Mechanics/BP_Player.BeginPuzzling` (`self.Player`) _asui_puzzle_border)
        (return _asui_puzzle_border)))))

(fn `RemoveKeyword`
  (params (Keyword :type String))
  (for (_array_element _array_index) (`self.Keywords`)
    (bind (_keyword _isunlocked _requiresfocus) (break `/Game/Mechanics/Structures/DAT_Keywords` _array_element))
    ;[1 1 1] Check if Exists
    (if (`KismetStringLibrary.EqualEqual_StrStr` _keyword Keyword)
      ;[1 1 1] Check if Already Owned
      (if _isunlocked
        (`KismetArrayLibrary.Array_Set` (`self.Keywords`) _array_index (make `/Game/Mechanics/Structures/DAT_Keywords` _keyword false _requiresfocus true))
        (return)))))

(fn `RequestItemDetails`
  (params (ItemID :type String) (ReturnCustomEmpty :type Boolean) (ReturnThisAsEmpty :type "/Game/Mechanics/Structures/DAT_ItemDetails Structure") (ReturnCustomError :type Boolean) (ReturnThisAsError :type "/Game/Mechanics/Structures/DAT_ItemDetails Structure"))
  (returns (OutItem :type "/Game/Mechanics/Structures/DAT_ItemDetails Structure"))
  (if (`KismetStringLibrary.EqualEqual_StrStr` ItemID)
    (if ReturnCustomEmpty
      (return ReturnThisAsEmpty)
      (else
        (return (make `/Game/Mechanics/Structures/DAT_ItemDetails` "-" "No Item" "There is no Item here" null null))))
    (else
      (for _array_element (`self.Items`)
        (if (`KismetStringLibrary.EqualEqual_StrStr` ItemID (`.ItemID_2_5C0729C0494167A6D9D0F69A6A48547F` (break `/Game/Mechanics/Structures/DAT_ItemDetails` _array_element)))
          (return _array_element)))
      (if ReturnCustomError
        (return ReturnThisAsError)
        (else
          (return (make `/Game/Mechanics/Structures/DAT_ItemDetails` "-" "Unnamed Item" "This item is undefined" null null)))))))

(fn `RequestItemDiscard`
  (params (Slot :type Integer))
  (returns (Outcome :type Boolean))
  (bind _outitem (`self.RequestItemDetails` (`|GetArrayItem` (`self.Inventory`) Slot)))
  (if (`.AllowManualDiscard_17_DDFC685744EEAAAB7AC3E9BCEE417411` (break `/Game/Mechanics/Structures/DAT_ItemDetails` _outitem))
    (`self.CallPlayerFunction` "NewEnumerator2" (break `/Game/Mechanics/Structures/DAT_ItemDetails` _outitem)))
  (return (`.AllowManualDiscard_17_DDFC685744EEAAAB7AC3E9BCEE417411` (break `/Game/Mechanics/Structures/DAT_ItemDetails` _outitem))))

(fn `RetreivePuzzleSolutionPiece`
  (params (PuzzleInt :type Integer) (PieceInt :type Integer))
  (returns (NewParam :type String))
  (bind _puzzle_numpadone (`self.Puzzle_NumPadOne`))
  (switch `int` PuzzleInt
    (:`Default`
      (return ""))
    (:`0`
      (switch `int` PieceInt
        (:`0`
          (bind _part (`/Game/Mechanics/Structures/I_PuzzleComponent.GetSolutionPart` _puzzle_numpadone "Thousands"))
          (return _part))
        (:`1`
          (bind _part_2 (`/Game/Mechanics/Structures/I_PuzzleComponent.GetSolutionPart` _puzzle_numpadone "Hundreds"))
          (return _part_2))
        (:`2`
          (bind _part_3 (`/Game/Mechanics/Structures/I_PuzzleComponent.GetSolutionPart` _puzzle_numpadone "Tens"))
          (return _part_3))
        (:`3`
          (bind _part_4 (`/Game/Mechanics/Structures/I_PuzzleComponent.GetSolutionPart` _puzzle_numpadone "Ones"))
          (return _part_4))))))

(fn `ReturnDiscussionViaDirectID`
  (params (RowName :type String))
  (returns (Discussion :type "/Game/Mechanics/Structures/DAT_Discussion Structure"))
  (bind _returnvalue (`|GetDataTableRow` (`self.DiscussionData`) (`KismetStringLibrary.Conv_StringToName` RowName))
    (:`then`
      (return _returnvalue))
    (:`RowNotFound`
      (`KismetSystemLibrary.PrintString` (`KismetStringLibrary.Concat_StrStr` RowName " - Dialogue not found!") true true (struct :`R` 1.0 :`G` 0.031298 :`A` 1.0) 15.0))))

(fn `ReturnDiscussionViaKeyword`
  (params (Keyword :type String) (Category :type String))
  (returns (Discussions :type "/Game/Mechanics/Structures/DAT_Discussion Structure"))
  (bind _returnvalue (`KismetStringLibrary.Replace` Keyword " " "_"))
  (bind _discussiondata (`self.DiscussionData`))
  (bind _discussiondata_2 (`self.DiscussionData`))
  (bind _returnvalue_2 (`KismetStringLibrary.Conv_StringToName` _returnvalue))
  (bind _returnvalue_3 (`KismetStringLibrary.Conv_StringToName` (`KismetStringLibrary.Concat_StrStr` _returnvalue "-" Category)))
  (if (`KismetStringLibrary.EqualEqual_StrStr` Category)
    (bind _returnvalue_4 (`DataTableFunctionLibrary.DoesDataTableRowExist` _discussiondata _returnvalue_2))
    (if _returnvalue_4
      (bind _returnvalue_5 (`|GetDataTableRow` _discussiondata_2 _returnvalue_2)
        (:`then`
          (return _returnvalue_5)))
      (else
        _))
    (else
      (bind _returnvalue_6 (`DataTableFunctionLibrary.DoesDataTableRowExist` _discussiondata _returnvalue_3))
      (if _returnvalue_6
        (bind _returnvalue_7 (`|GetDataTableRow` _discussiondata_2 _returnvalue_3)
          (:`then`
            (return _returnvalue_7)))
        (else
          _))))
  (return))

(fn `ReturnObjectives`
  (returns (Formatted :type "Array of String"))
  (locals (Final :type "Array of String") (ObjArray :type "Array of String"))
  (bind _objarray (`local.ObjArray`))
  (for _array_element (`self.Objectives`)
    (`KismetArrayLibrary.Array_Add` _objarray (`.ObjectiveName_2_D0414EDB40CFE06FF418B498F307FF01` (break `/Game/Mechanics/Structures/DAT_Objectives` _array_element))))
  (for (_array_element_2 _array_index) _objarray
    (if (> _array_index 0)
      (bind _returnvalue (`KismetStringLibrary.Concat_StrStr` "- " _array_element_2))
      (`KismetArrayLibrary.Array_Add` (`local.Final`) _returnvalue)
      (else
        (set `local.Final` (`|MakeArray` _returnvalue)))))
  (return (`local.Final`)))

(fn `SaveLoad`
  (params (Load :type Boolean) (Slot :type Integer) (LevelOnly :type Boolean))
  (bind _assave_state_info (cast `/Game/Mechanics/SaveStateInfo` (`GameplayStatics.GetPlayerState` 0))
    (:`then`
      (if Load
        (`/Game/Mechanics/SaveStateInfo.LoadGame` _assave_state_info Slot LevelOnly)
        (else
          (`/Game/Mechanics/SaveStateInfo.SaveGame` _assave_state_info Slot)
          (set `/Game/Mechanics/HorrorSiloGameInstance.ShouldLoad` true (cast `/Game/Mechanics/HorrorSiloGameInstance` (`GameplayStatics.GetGameInstance`) :!pure true)))))
    (:`CastFailed`
      (`KismetSystemLibrary.PrintString` "Oh no"))))

(fn `TryInspectItem`
  (params (Slot :type Integer) (Item :type "Actor Object Reference"))
  (bind _output (`|GetArrayItem` (`self.Inventory`) Slot))
  (bind _asi_item (cast `/Game/Mechanics/Structures/I_Item` Item)
    (:`then`
      (bind _itemid (`/Game/Mechanics/Structures/I_Item.GetItemID` _asi_item))
      (bind _outitem (`self.RequestItemDetails` _itemid))
      (bind _returnvalue (`KismetSystemLibrary.LoadClassAsset_Blocking` (`.ActorOfItem_15_081B249B4C6B7AD660E38DA388C4E05B` (break `/Game/Mechanics/Structures/DAT_ItemDetails` _outitem))))
      (bind _returnvalue_2 (`|GenericCreateObject` _returnvalue))
      (bind _asi_item_2 (cast `/Game/Mechanics/Structures/I_Item` _returnvalue_2))
      (bind (_2drepresentation _3dreprenetation) (`/Game/Mechanics/Structures/I_Item.RequestedInspect` _asi_item_2))
      (`/Game/Mechanics/BP_Player.BeginInspect` :`self` (`self.Player`) :`Mesh` _3dreprenetation :`Widget` _2drepresentation))
    (:`CastFailed`
      (`KismetSystemLibrary.PrintString` _output)
      (bind _outitem_2 (`self.RequestItemDetails` _output))
      (bind _returnvalue_3 (`KismetSystemLibrary.LoadClassAsset_Blocking` (`.ActorOfItem_15_081B249B4C6B7AD660E38DA388C4E05B` (break `/Game/Mechanics/Structures/DAT_ItemDetails` _outitem_2))))
      (bind _returnvalue_4 (`|GenericCreateObject` (`self.Player`) _returnvalue_3))
      (bind _asi_item_3 (cast `/Game/Mechanics/Structures/I_Item` _returnvalue_4))
      (bind (_2drepresentation_2 _3dreprenetation_2) (`/Game/Mechanics/Structures/I_Item.RequestedInspect` _asi_item_3))
      (`/Game/Mechanics/BP_Player.BeginInspect` (`self.Player`) _outitem_2 _3dreprenetation_2 _2drepresentation_2 false null "" ""))))

(fn `TryInspectNonPickableItem`
  (params (Name :type String))
  (bind _returnvalue (`|GetDataTableRow` (`self.InspectData`) (`KismetStringLibrary.Conv_StringToName` Name))
    (:`then`
      (bind (_name _description _image) (break `/Game/Mechanics/Structures/DAT_InspectableDetails` _returnvalue))
      (`/Game/Mechanics/BP_Player.BeginInspect` :`self` (`self.Player`) :`IgnoreVars` true :`Image` _image :`Inspectable` _name :`Description` _description))))

(fn `UserConstructionScript`
  (bind _returnvalue (`GameplayStatics.GetStreamingLevel` "Hub_01_SD"))
  (bind _objectivedata (`self.ObjectiveData`))
  (bind _keyworddata (`self.KeywordData`))
  (bind _itemdata (`self.ItemData`))
  (if (== (`KismetArrayLibrary.Array_Length` (`self.Items`)) 0)
    (`|ExecutionSequence`
      (:`then_0`
        (bind _outrownames (`DataTableFunctionLibrary.GetDataTableRowNames` _itemdata))
        (for _array_element _outrownames
          (bind _returnvalue_2 (`|GetDataTableRow` _itemdata _array_element)
            (:`then`
              (`KismetArrayLibrary.Array_Add` (`self.Items`) _returnvalue_2)))))
      (:`then_1`
        (bind _outrownames_2 (`DataTableFunctionLibrary.GetDataTableRowNames` _objectivedata))
        (for _array_element_2 _outrownames_2
          (bind _returnvalue_3 (`|GetDataTableRow` _objectivedata _array_element_2)
            (:`then`
              (bind (_objectivename _isdelirius _markcompletedon) (break `/Game/Mechanics/Structures/DAT_Objectives` _returnvalue_3))
              (if (< _markcompletedon 0)
                (`self.AddRemoveObjectives` _objectivename true))))))
      (:`then_2`
        (bind _outrownames_3 (`DataTableFunctionLibrary.GetDataTableRowNames` _keyworddata))
        (for _array_element_3 _outrownames_3
          (bind _returnvalue_4 (`|GetDataTableRow` _keyworddata _array_element_3)
            (:`then`
              (`KismetArrayLibrary.Array_Add` (`self.Keywords`) _returnvalue_4)))))
      (:`then_3`
        (set `self.GameSessionSeed` (`KismetMathLibrary.RandomIntegerInRange` 10000000 99999999))
        (`/Engine/EditorBlueprintResources/StandardMacros.IsValid` _returnvalue
          (:`Is Valid`
            (add `LevelStreaming.OnLevelLoaded` _returnvalue (`|CreateDelegate` :!event `GM_Silo13_AutoGenFunc`))))))))