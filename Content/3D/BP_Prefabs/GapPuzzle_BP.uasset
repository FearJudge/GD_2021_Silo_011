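; Gap puzzle interactable that lets the player cross a gap by using the required puzzle item on it to place a plank.
; DoAction checks the item, calls the player through GM_Silo13, toggles DoorState, updates InteractableItem's save state and plays a sound; wrong items show a message.
; SetPlank toggles plank visibility and swaps collision between Blocker and Cube.
; SetStateBasedOnSaveData reapplies the plank state from saved data.
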(event `self.ReceiveBeginPlay`
  (`self.SetPlank` false)
  (bind _asgm_silo_13 (cast `/Game/Mechanics/GM_Silo13` (`GameplayStatics.GetGameMode`)))
  (set `self.As GM Silo 13` _asgm_silo_13))

(event `/Game/Mechanics/Structures/I_Implementable.DoAction`
  (params (UsedItem :type String))
  (bind _puzzleitem (`self.PuzzleItem`))
  (bind _interactableitem (`self.InteractableItem`))
  (bind _as_gm_silo_13 (`self.As GM Silo 13`))
  (bind _interactableitem_2 (`self.InteractableItem`))
  (if (`KismetStringLibrary.EqualEqual_StrStr` UsedItem _puzzleitem)
    (`/Game/Mechanics/BP_Player.ToggleINVENTORY` (`/Game/Mechanics/GM_Silo13.Player` _as_gm_silo_13) false true null)
    (`/Game/Mechanics/GM_Silo13.CallPlayerFunction` _as_gm_silo_13 "NewEnumerator2" _puzzleitem null)
    (set `/Game/Mechanics/InteractableItem.InteractDisplayType` "" (`self.InteractableItem`))
    (`|ExecutionSequence`
      (:`then_0`
        (`|ExecutionSequence`
          (:`then_0`
            ;[1 1 1] SaveLogic
            (bind _output_get (set `self.DoorState` (not (`self.DoorState`))))
            (if _output_get
              (set `/Game/Mechanics/InteractableItem.InteractDisplayType` "Close" _interactableitem_2)
              (set `/Game/Mechanics/InteractableItem.SavableState` "NewEnumerator7" _interactableitem)
              (set `/Game/Mechanics/InteractableItem.ValidDirection` "NewEnumerator0" _interactableitem)
              (`/Game/Mechanics/InteractableItem.Set Enabled` (`self.InteractableItem`) false)
              (else
                (set `/Game/Mechanics/InteractableItem.InteractDisplayType` "Open" _interactableitem_2)
                (set `/Game/Mechanics/InteractableItem.SavableState` "NewEnumerator3" _interactableitem))))
          (:`then_1`
            (`self.SetPlank` (`self.DoorState`)))))
      (:`then_1`
        (`GameplayStatics.PlaySoundAtLocation` "/Game/Audio/SFX/FILMCOW/CUE_Item.CUE_Item" (`self.K2_GetActorLocation`) (struct) 1.0 1.0 0.0 null null null null)))
    (elif (`KismetStringLibrary.EqualEqual_StrStr` UsedItem)
      (`/Game/Mechanics/GM_Silo13.CallPlayerFunction` _as_gm_silo_13 "NewEnumerator12" "Choose an item to use." null)
      (else
        (`/Game/Mechanics/GM_Silo13.CallPlayerFunction` _as_gm_silo_13 "NewEnumerator12" "Cannot use this item here." null)))))

(fn `ComponentIsNotTraceable`
  (params (Hit :type "ActorComponent Object Reference"))
  (returns (Blocked :type Boolean))
  (return (== Hit null)))

(fn `GetInteractableItem`
  (returns (Item :type "/Game/Mechanics/InteractableItem Object Reference"))
  (return (`self.InteractableItem`)))

(fn `GetPivotForDir`
  (returns (HasDifferentPivot :type Boolean) (NewPivot :type "Vector Structure"))
  (return false (0.0 0.0 0.0)))

(fn `SetPlank`
  (params (State :type Boolean))
  (bind _staticmesh (`self.StaticMesh`))
  (bind _blocker (`self.Blocker`))
  (bind _cube (`self.Cube`))
  (if State
    (`PrimitiveComponent.SetCollisionEnabled` _staticmesh "NoCollision")
    (`SceneComponent.SetVisibility` _staticmesh true false)
    (`PrimitiveComponent.SetCollisionEnabled` _blocker "NoCollision")
    (`PrimitiveComponent.SetCollisionEnabled` _cube "QueryAndPhysics")
    (else
      (`PrimitiveComponent.SetCollisionEnabled` _staticmesh "NoCollision")
      (`SceneComponent.SetVisibility` _staticmesh false false)
      (`PrimitiveComponent.SetCollisionEnabled` _blocker "QueryAndPhysics")
      (`PrimitiveComponent.SetCollisionEnabled` _cube "NoCollision"))))

(fn `SetStateBasedOnSaveData`
  (params (StateToFollow :type "/Game/Mechanics/Structures/ENUM_SavedState Enum" :default "NewEnumerator0"))
  (returns (Implemented :type Boolean))
  (if (`|EnumEquality` StateToFollow "NewEnumerator3")
    (set `/Game/Mechanics/InteractableItem.ValidDirection` "NewEnumerator0" (`self.InteractableItem`))
    (`self.SetPlank` true)
    (return true)
    (else
      (`self.SetPlank` false)
      (return true))))

(fn `UserConstructionScript`)