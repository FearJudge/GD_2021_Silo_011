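; BP_DaysOfAccidents is a days-of-accidents display that shows a puzzle solution as its record number.
; One tick after BeginPlay, it gets puzzle 3 from GM_Silo13 and joins the hundreds, tens and ones solution parts into the RecordT text.
; CurrentT shows a random count 100 to 200 below that record, so the solution is always the higher number.
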(event `self.ReceiveBeginPlay`
  (bind _asgm_silo_13 (cast `/Game/Mechanics/GM_Silo13` (`GameplayStatics.GetGameMode`)))
  (`KismetSystemLibrary.DelayUntilNextTick`)
  (bind _puzzle (`/Game/Mechanics/GM_Silo13.RetrievePuzzle` _asgm_silo_13 3))
  (bind _part (`/Game/Mechanics/Structures/I_PuzzleComponent.GetSolutionPart` _puzzle "Hundreds"))
  (bind _part_2 (`/Game/Mechanics/Structures/I_PuzzleComponent.GetSolutionPart` _puzzle "Tens"))
  (bind _part_3 (`/Game/Mechanics/Structures/I_PuzzleComponent.GetSolutionPart` _puzzle "Ones"))
  (bind _returnvalue (`KismetStringLibrary.Concat_StrStr` _part _part_2 _part_3))
  (`TextRenderComponent.K2_SetText` (`self.RecordT`) (`KismetTextLibrary.Conv_StringToText` _returnvalue))
  (bind _returnvalue_2 (`KismetStringLibrary.Conv_StringToInt` _returnvalue))
  (`TextRenderComponent.K2_SetText` (`self.CurrentT`) (`KismetTextLibrary.Conv_IntToText` (`KismetMathLibrary.RandomIntegerInRange` (- _returnvalue_2 200) (- _returnvalue_2 100)))))

(fn `UserConstructionScript`)