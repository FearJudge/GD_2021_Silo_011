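; Spline tool actor that builds a pipe from repeated spline meshes along its spline in the construction script, with optional start and end caps.
; PipeSetup sizes segments by the mesh's X bounds times actor scale, clamping tangents to that length; FullLengthMesh omits the final partial segment.
; Segments take a material and optional collision.
; Cap static meshes align to the first and last segment's position and tangent, plus a rotation offset.
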(fn `EndCapSetup`
  (bind _splinemeshes (`self.SplineMeshes`))
  (bind _output (`|GetArrayItem` _splinemeshes (- (`KismetArrayLibrary.Array_Length` _splinemeshes) 1)))
  (bind (_returnvalue_roll _returnvalue_pitch _returnvalue_yaw) (`KismetMathLibrary.BreakRotator` (`KismetMathLibrary.Conv_VectorToRotator` (`SplineMeshComponent.GetEndTangent` _output))))
  (bind _returnvalue (`AddComponent|NODE_AddStaticMeshComponent-4`))
  (`StaticMeshComponent.SetStaticMesh` _returnvalue (`self.EndCap`))
  (`PrimitiveComponent.SetMaterial` _returnvalue 0 (`self.EndCapMaterial`))
  (`SceneComponent.K2_AttachToComponent` _returnvalue (`self.Spline`) "None" "KeepRelative" "KeepRelative" "KeepRelative" true)
  (`SceneComponent.K2_SetRelativeLocationAndRotation` _returnvalue (`SplineMeshComponent.GetEndPosition` _output) (`KismetMathLibrary.ComposeRotators` (`KismetMathLibrary.MakeRotator` (`SplineMeshComponent.GetEndRoll` _output) (* _returnvalue_pitch -1.0) _returnvalue_yaw) (`self.EndCapRotation`)) false false)
  (return))

(fn `GetEndPosAndTangent`
  (returns (Location :type "Vector Structure") (Tangent :type "Vector Structure"))
  (bind _length (`self.Length`))
  (bind _spline (`self.Spline`))
  (bind _returnvalue (* (+ (`self.Index`) 1) (`self.Length`)))
  (return (`SplineComponent.GetLocationAtDistanceAlongSpline` _spline _returnvalue "Local") (`KismetMathLibrary.ClampVectorSize` (`SplineComponent.GetTangentAtDistanceAlongSpline` _spline _returnvalue "Local") _length _length)))

(fn `GetStartPosAndTangent`
  (returns (Location :type "Vector Structure") (Tangent :type "Vector Structure"))
  (bind _length (`self.Length`))
  (bind _spline (`self.Spline`))
  (bind _returnvalue (* (`self.Index`) (`self.Length`)))
  (return (`SplineComponent.GetLocationAtDistanceAlongSpline` _spline _returnvalue "Local") (`KismetMathLibrary.ClampVectorSize` (`SplineComponent.GetTangentAtDistanceAlongSpline` _spline _returnvalue "Local") _length _length)))

(fn `PipeSetup`
  (bind _returnvalue_x (`KismetMathLibrary.BreakVector` (`self.GetActorScale3D`)))
  (bind (_min _max) (break `Box` (`StaticMesh.GetBoundingBox` (`self.PipeMesh`))))
  (`KismetArrayLibrary.Array_Clear` (`self.SplineMeshes`))
  ;[1 1 1] Scaling
  (set `self.Length` (* _returnvalue_x (.x (- _max _min))))
  ;[1 1 1] Enable full length mesh
  (if (`self.FullLengthMesh`)
    ;[1 1 1] Show only full length meshes
    (for _index (range (`KismetMathLibrary.FTrunc` (/ (`SplineComponent.GetSplineLength` (`self.Spline`)) (`self.Length`))))
      (set `self.Index` _index)
      ;[1 1 1] Add mesh to spline
      (bind _returnvalue (`AddComponent|NODE_AddSplineMeshComponent-5` :!label _label))
      (`KismetArrayLibrary.Array_Set` (`self.SplineMeshes`) (`self.Index`) _returnvalue true)
      (`StaticMeshComponent.SetStaticMesh` _returnvalue (`self.PipeMesh`))
      (`PrimitiveComponent.SetMaterial` _returnvalue 0 (`self.PipeMeshMaterial`))
      (`SplineMeshComponent.SetForwardAxis` _returnvalue "X" true)
      (`SceneComponent.K2_AttachToComponent` _returnvalue (`self.Spline`) "None" "KeepRelative" "KeepRelative" "KeepRelative" true)
      (bind (_location _tangent) (`self.GetStartPosAndTangent`))
      (bind (_location_2 _tangent_2) (`self.GetEndPosAndTangent`))
      (`SplineMeshComponent.SetStartAndEnd` _returnvalue _location _tangent _location_2 _tangent_2 true)
      (if (`self.EnableCollision`)
        (`PrimitiveComponent.SetCollisionEnabled` _returnvalue (`self.CollisionType`))))
    (return)
    (else
      (for _index_2 (range (+ (`KismetMathLibrary.FTrunc` (/ (`SplineComponent.GetSplineLength` (`self.Spline`)) (`self.Length`))) 1))
        (set `self.Index` _index_2)
        (goto _label))
      (return))))

(fn `StartCapSetup`
  (bind _output (`|GetArrayItem` (`self.SplineMeshes`)))
  (bind (_returnvalue_roll _returnvalue_pitch _returnvalue_yaw) (`KismetMathLibrary.BreakRotator` (`KismetMathLibrary.Conv_VectorToRotator` (`SplineMeshComponent.GetStartTangent` _output))))
  (bind _returnvalue (`AddComponent|NODE_AddStaticMeshComponent-3`))
  (`StaticMeshComponent.SetStaticMesh` _returnvalue (`self.StartCap`))
  (`PrimitiveComponent.SetMaterial` _returnvalue 0 (`self.StartCapMaterial`))
  (`SceneComponent.K2_AttachToComponent` _returnvalue (`self.Spline`) "None" "KeepRelative" "KeepRelative" "KeepRelative" true)
  (`SceneComponent.K2_SetRelativeLocationAndRotation` _returnvalue (`SplineMeshComponent.GetStartPosition` _output) (`KismetMathLibrary.ComposeRotators` (`KismetMathLibrary.MakeRotator` (`SplineMeshComponent.GetStartRoll` _output) _returnvalue_pitch _returnvalue_yaw) (`self.StartCapRotation`)) false false)
  (return))

(fn `UserConstructionScript`
  (`self.PipeSetup`)
  (if (`self.EnableStartCap`)
    (`self.StartCapSetup`))
  (if (`self.EnableEndCap`)
    (`self.EndCapSetup`)))