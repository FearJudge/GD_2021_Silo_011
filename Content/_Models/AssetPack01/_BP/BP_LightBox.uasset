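; Light box interactable actor that opens a light puzzle interface through the Silo13 game mode when used.
; It binds to the puzzle's completion event to mark its InteractableItem's savable state as solved.
; Loading a solved state sets SolveOnInteract, so the next interaction solves the puzzle through the game mode before opening the interface.
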(event `/Game/Mechanics/Structures/I_Implementable.DoAction`
  (bind _asgm_silo_13 (cast `/Game/Mechanics/GM_Silo13` (`GameplayStatics.GetGameMode`)))
  (if (`self.SolveOnInteract`)
    (`/Game/Mechanics/UIPieces/UI_4-DigitLock.SolvePuzzle` (`/Game/Mechanics/GM_Silo13.PuzzleLightPuzzleOne` _asgm_silo_13)))
  (bind _puzzle (`/Game/Mechanics/GM_Silo13.OpenPuzzleInterface` _asgm_silo_13 1))
  (add `/Game/Mechanics/UIPieces/UI_PuzzleBorder.PuzzleCompleted` _puzzle (delegate `SetPuzzleCompletion`)))

(event `SetPuzzleCompletion`
  (set `/Game/Mechanics/InteractableItem.SavableState` "NewEnumerator10" (`self.InteractableItem`)))

(fn `ComponentIsNotTraceable`
  (params (Hit :type "ActorComponent Object Reference"))
  (returns (Blocked :type Boolean))
  (return false))

(fn `GetInteractableItem`
  (returns (Item :type "/Game/Mechanics/InteractableItem Object Reference"))
  (return (`self.InteractableItem`)))

(fn `SetStateBasedOnSaveData`
  (params (StateToFollow :type "/Game/Mechanics/Structures/ENUM_SavedState Enum" :default "NewEnumerator0"))
  (returns (Implemented :type Boolean))
  (switch `/Game/Mechanics/Structures/ENUM_SavedState` StateToFollow
    (:`NewEnumerator10`
      (set `self.SolveOnInteract` true)
      (return true))))

(fn `UserConstructionScript`)