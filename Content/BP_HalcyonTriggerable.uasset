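; BP_HalcyonTriggerable is a flag-triggered rect light actor that starts dark unless its State is set.
; The construction script caches the light's intensity, and BeginPlay zeroes it when State is false.
; It binds Activate to the GM_Silo13 game mode's kill-actor-on-flag event.
; When the flag matches OnTrigger, Activate restores the intensity and adds Distort and BlueLight actor tags.
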(event `self.ReceiveBeginPlay`
  (`|ExecutionSequence`
    (:`then_0`
      (if (not (`self.State`))
        (`LightComponent.SetIntensity` (`self.RectLight`) 0.0)))
    (:`then_1`
      (bind _asgm_silo_13 (cast `/Game/Mechanics/GM_Silo13` (`GameplayStatics.GetGameMode`)))
      (add `/Game/Mechanics/GM_Silo13.KillActorOnFlag` _asgm_silo_13 (delegate `Activate`)))))

(event `Activate`
  (params (Flag :type String))
  (bind _tags (`self.Tags`))
  (if (`KismetStringLibrary.EqualEqual_StrStr` Flag (`self.OnTrigger`))
    (`LightComponent.SetIntensity` (`self.RectLight`) (`self.Intensity`))
    (`KismetArrayLibrary.Array_AddUnique` _tags "Distort")
    (`KismetArrayLibrary.Array_AddUnique` _tags "BlueLight")))

(fn `UserConstructionScript`
  (set `self.Intensity` (`LightComponentBase.Intensity` (`self.RectLight`))))