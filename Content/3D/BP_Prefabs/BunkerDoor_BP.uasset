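; Interactable bunker door that toggles open and closed with a metal door sound.
; DoAction ignores repeat calls mid-motion and plays one timeline forward or in reverse to drive the door swing, latch rods, handle and spinning wheel.
; On finish it flips DoorState and updates the InteractableItem's prompt and savable state.
; SetStateBasedOnSaveData only returns false, so it restores no saved state.
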(event `/Game/Mechanics/Structures/I_Implementable.DoAction`
  (bind _doorstate (`self.DoorState`))
  (bind _interactableitem (`self.InteractableItem`))
  (bind _interactableitem_2 (`self.InteractableItem`))
  (if (not (`self.In Progress`))
    (set `self.In Progress` true)
    (set `/Game/Mechanics/InteractableItem.InteractDisplayType` "" (`self.InteractableItem`))
    (`|ExecutionSequence`
      (:`then_0`
        (if _doorstate
          (bind (_direction _door_locks _door_latches _door_swing) (`Timeline|Door State Animation` :!via `ReverseFromEnd` :!label _label)
            (:`Update`
              ;[1 1 1] ANIMATION
              (`SceneComponent.K2_SetRelativeRotation` (`self.Bunker Door`) (`KismetMathLibrary.MakeRotator` 0.0 0.0 (* _door_swing 90.0)) false false) ; Wheel
              (bind _returnvalue (* _door_latches 10.0))
              (`SceneComponent.K2_SetRelativeLocation` (`self.Rod Top Right`) (`KismetMathLibrary.MakeVector` _returnvalue) false false) ; Right-side Bar_1
              (`SceneComponent.K2_SetRelativeLocation` (`self.Rod Bottom Right`) (`KismetMathLibrary.MakeVector` _returnvalue) false false) ; Right-side Bar_2
              (bind _returnvalue_2 (* _returnvalue -1.0))
              (`SceneComponent.K2_SetRelativeLocation` (`self.Rod Top Left`) (`KismetMathLibrary.MakeVector` _returnvalue_2) false false) ; Left-side Bar_1
              (`SceneComponent.K2_SetRelativeLocation` (`self.Rod Bottom Left`) (`KismetMathLibrary.MakeVector` _returnvalue_2) false false) ; Left-side Bar_2
              (bind _returnvalue_3 (* _door_latches 20.0))
              (`SceneComponent.K2_SetRelativeLocation` (`self.Rod Bottom`) (`KismetMathLibrary.MakeVector` 0.0 0.0 (* _returnvalue_3 -1.0)) false false) ; Downward Bar_1
              (`SceneComponent.K2_SetRelativeLocation` (`self.Rod Top`) (`KismetMathLibrary.MakeVector` 0.0 0.0 _returnvalue_3) false false) ; Upward Bar_2
              (`SceneComponent.K2_SetRelativeLocation` (`self.Handle`) (`KismetMathLibrary.MakeVector` (* _door_locks -10.0)) false false) ; Latch
              (`SceneComponent.K2_SetRelativeRotation` (`self.Wheel`) (`KismetMathLibrary.MakeRotator` 0.0 (* _door_locks 360.0)) false false))
            (:`Finished`
              ;[1 1 1] SaveLogic
              (bind _output_get (set `self.DoorState` (not _doorstate)))
              (set `self.In Progress` false)
              (if _output_get
                (set `/Game/Mechanics/InteractableItem.InteractDisplayType` "Close" _interactableitem_2)
                (set `/Game/Mechanics/InteractableItem.SavableState` "NewEnumerator6" _interactableitem)
                (else
                  (set `/Game/Mechanics/InteractableItem.InteractDisplayType` "Open" _interactableitem_2)
                  (set `/Game/Mechanics/InteractableItem.SavableState` "NewEnumerator5" _interactableitem)))))
          (else
            (goto _label :!via `PlayFromStart`))))
      (:`then_1`
        (`GameplayStatics.PlaySoundAtLocation` "/Game/Audio/SFX/DOOR/BIG2/OPEN/Cue_MetalDoor.Cue_MetalDoor" (`self.K2_GetActorLocation`) (struct) 1.0 1.0 0.0 null null null null)))))

(fn `ComponentIsNotTraceable`
  (params (Hit :type "ActorComponent Object Reference"))
  (returns (Blocked :type Boolean))
  (return (== Hit (`self.tunnel_square_doorway_bunkerdoor`))))

(fn `GetInteractableItem`
  (returns (Item :type "/Game/Mechanics/InteractableItem Object Reference"))
  (return (`self.InteractableItem`)))

(fn `SetStateBasedOnSaveData`
  (params (StateToFollow :type "/Game/Mechanics/Structures/ENUM_SavedState Enum" :default "NewEnumerator0"))
  (returns (Implemented :type Boolean))
  (return false))

(fn `UserConstructionScript`)