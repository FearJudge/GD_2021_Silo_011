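; BP_Lever is an interactable lever actor that toggles between on and off, with an optional one-time use.
; DoAction flips the Set flag, then updates the InteractableItem component's savable state and "Switch On"/"Switch Off" prompt, or disables it when OneTime.
; It exposes the component through GetInteractableItem and reports itself as non-traceable.
; SetStateBasedOnSaveData only returns true for default and interacted-enabled states, without restoring the lever.
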(event `/Game/Mechanics/Structures/I_Implementable.DoAction`
  (bind _interactableitem (`self.InteractableItem`))
  (bind _output_get (set `self.Set` (not (`self.Set`))))
  (if _output_get
    (if (`self.OneTime`)
      (set `/Game/Mechanics/InteractableItem.SavableState` "NewEnumerator7" _interactableitem)
      (`/Game/Mechanics/InteractableItem.Set Enabled` (`self.InteractableItem`) false)
      (else
        (set `/Game/Mechanics/InteractableItem.SavableState` "NewEnumerator6" _interactableitem)
        (set `/Game/Mechanics/InteractableItem.InteractDisplayType` "Switch Off" _interactableitem)))
    (else
      (set `/Game/Mechanics/InteractableItem.SavableState` "NewEnumerator0" _interactableitem)
      (set `/Game/Mechanics/InteractableItem.InteractDisplayType` "Switch On" _interactableitem))))

(fn `ComponentIsNotTraceable`
  (params (Hit :type "ActorComponent Object Reference"))
  (returns (Blocked :type Boolean))
  (return false))

(fn `GetInteractableItem`
  (returns (Item :type "/Game/Mechanics/InteractableItem Object Reference"))
  (return (`self.InteractableItem`)))

(fn `SetStateBasedOnSaveData`
  (params (StateToFollow :type "/Game/Mechanics/Structures/ENUM_SavedState Enum" :default "NewEnumerator0"))
  (returns (Implemented :type Boolean))
  (switch `/Game/Mechanics/Structures/ENUM_SavedState` StateToFollow
    (:`NewEnumerator0`
      (return true))
    (:`NewEnumerator6`
      (return true))))

(fn `UserConstructionScript`)