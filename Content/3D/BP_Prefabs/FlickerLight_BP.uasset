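; FlickerLight_BP is a spotlight prefab that flickers at random intervals when it starts switched on.
; The construction script applies the color, on/off switch and intensity variables to the SpotLight.
; On BeginPlay, a visible light starts a random-delay timer that plays a random-length timeline, randomizing intensity on every update.
; When the timeline finishes, it restores the set intensity and schedules the next flicker, repeating indefinitely.
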(event `self.ReceiveBeginPlay`
  (if (`SceneComponent.bVisible` (`self.SpotLight`))
    (`self.initiateFlicker`)))

(event `initiateFlicker`
  (bind _returnvalue (`KismetSystemLibrary.K2_SetTimer` null "flickerLight" (`KismetMathLibrary.RandomFloatInRange` 2.0 10.0)))
  (set `self.flickerTimer` _returnvalue))

(event `flickerLight`
  (`TimelineComponent.SetTimelineLength` (`self.flickerTime`) (`KismetMathLibrary.RandomFloatInRange` 2.0 10.0))
  (`Timeline|flickerTime` :!via `PlayFromStart`
    (:`Update`
      (`LightComponent.SetIntensity` (`self.SpotLight`) (`KismetMathLibrary.RandomFloatInRange` 10000.0 (`self.lightIntensity`))))
    (:`Finished`
      (`LightComponent.SetIntensity` (`self.SpotLight`) (`self.lightIntensity`))
      (`KismetSystemLibrary.K2_ClearAndInvalidateTimerHandle` (`self.flickerTimer`))
      (`self.initiateFlicker`))))

(fn `UserConstructionScript`
  (bind _spotlight (`self.SpotLight`))
  (bind _output_get (set `self.lightColor` (`self.lightColor`)))
  (`LightComponent.SetLightColor` _spotlight _output_get true)
  (`SceneComponent.SetVisibility` _spotlight (`self.lightSwitch`) false)
  (bind _output_get_2 (set `self.lightIntensity` (`self.lightIntensity`)))
  (`LightComponent.SetIntensity` (`self.SpotLight`) _output_get_2))